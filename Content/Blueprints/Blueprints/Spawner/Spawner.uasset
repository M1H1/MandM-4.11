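; Spawner actor that keeps a single AI follower character alive within the radius of its sphere component.
; Each Tick, when SpawnedAi is no longer valid, it spawns a Ue4ASP_Character running AI_Follower_BT at a random reachable point in that radius and stores it.
; An unconnected copy of the spawn chain, which also sets Health to 100, never executes.
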(event EventBeginPlay)

(event EventTick
  (params (DeltaSeconds :type Float%20%28single-precision%29))
  (Utilities|IsValid (Variables|Default|GetSpawned%20Ai)
    (:Is%20Not%20Valid
      (bind _returnvalue (AI|SpawnAIFromClass "/Game/Ai/BasicAiEnemy/Ue4ASP_Character.Ue4ASP_Character_C" "/Game/Ai/BasicAiEnemy/AiClasses/AI_Follower_BT.AI_Follower_BT" (AI|Navigation|GetRandomReachablePointinRadius (Transformation|GetActorLocation) (Variables|/Script/Engine.SphereComponent|GetSphereRadius (Variables|Default|GetSphere))) "0, 0, 0" true))
      (Variables|Default|SetSpawned%20Ai _returnvalue))))

(fn ConstructionScript)